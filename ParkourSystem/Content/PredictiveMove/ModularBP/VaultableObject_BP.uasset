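; VaultableObject_BP is an obstacle the player can vault over, supplying the direction and endpoints of the vault.
; FindFaceDirection tests front and back arrows against a minimum dot to decide whether vaulting is allowed and which way.
; Start and end are the points closest to the player character on the opposing front and back splines, lowered by a Z offset.
; GetType reports a fixed enum type, and the event graph is unused.
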(fn `GetType`
  (returns (NewParam :type "/Game/PredictiveMove/MoveableObjectType_Enum Enum"))
  (return "NewEnumerator1"))

(fn `GetVaultDirectionAndLocations`
  (params (MinDot :type "Float (double-precision)") (ZOffset :type "Float (double-precision)"))
  (returns (`CanVault?` :type Boolean) (StartLocaion :type "Vector Structure") (EndLocation :type "Vector Structure") (DirectionRotation :type "Rotator Structure"))
  (bind _zoffset (`local.ZOffset`))
  (bind (_facing_ _facingarrow _isfrontarrow) (`self.FindFaceDirection` (`self.FrontArrow`) (`self.BackArrow`) (`local.MinDot`)))
  (bind _returnvalue (`self.K2_GetActorLocation` (`GameplayStatics.GetPlayerCharacter` 0)))
  ;[1 1 1] Use the FindFaceDirection function to return the target direction. The start and end locations are found on the spline relative to the target direction.
  (return _facing_ (- (`SplineComponent.FindLocationClosestToWorldLocation` (select `bool` _isfrontarrow :`false` (`self.FrontSpline`) :`true` (`self.BackSpline`)) _returnvalue "World") (`KismetMathLibrary.MakeVector` 0.0 0.0 _zoffset)) (- (`SplineComponent.FindLocationClosestToWorldLocation` (select `bool` _isfrontarrow :`false` (`self.BackSpline`) :`true` (`self.FrontSpline`)) _returnvalue "World") (`KismetMathLibrary.MakeVector` 0.0 0.0 _zoffset)) (`KismetMathLibrary.MakeRotFromX` (`SceneComponent.GetForwardVector` _facingarrow))))

(fn `UserConstructionScript`
  (`parent.UserConstructionScript`))