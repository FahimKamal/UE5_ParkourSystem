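; MoveableObject_BP is a modular base actor for objects in the predictive movement system, exposing land position, peak position, spline and type getters with simple or placeholder defaults.
; The construction script places the LandPosition component and spawns a static mesh component from configurable mesh, scale and rotation, preserving its materials.
; FindFaceDirection compares the player-to-object direction against front and back arrows by dot product, returning whether the player faces either and which one.
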(fn `FindFaceDirection`
  (params (FrontArrow :type "SceneComponent Object Reference") (BackArrow :type "SceneComponent Object Reference") (MinDot :type "Float (double-precision)"))
  (returns (`Facing?` :type Boolean) (FacingArrow :type "SceneComponent Object Reference") (IsFrontArrow :type Boolean))
  (bind _returnvalue (`KismetMathLibrary.GetForwardVector` (`KismetMathLibrary.FindLookAtRotation` (`self.K2_GetActorLocation` (`GameplayStatics.GetPlayerCharacter` 0)) (`self.K2_GetActorLocation`))))
  (bind _returnvalue_2 (> (`KismetMathLibrary.Dot_VectorVector` (`SceneComponent.GetForwardVector` FrontArrow) _returnvalue) (`local.MinDot`)))
  ;[1 1 1] For objects where the player must be facing a certain direction to it, find if the player is and which arrow they are facing.
  (return (or _returnvalue_2 (> (`KismetMathLibrary.Dot_VectorVector` (`SceneComponent.GetForwardVector` BackArrow) _returnvalue) (`local.MinDot`))) (select `bool` _returnvalue_2 :`false` (`local.BackArrow`) :`true` (`local.FrontArrow`)) _returnvalue_2))

(fn `GetLandPosition`
  (returns (Location :type "Vector Structure"))
  ;[1 1 1] By default, this function returns the world location of the lland scene component.
  (return (`SceneComponent.K2_GetComponentLocation` (`self.LandPosition`))))

(fn `GetPeakPosition`
  (returns (Location :type "Vector Structure"))
  (return (0.0 0.0 0.0)))

(fn `GetSpline`
  (returns (Spline :type "SplineComponent Object Reference"))
  (return null))

(fn `GetType`
  (returns (NewParam :type "/Game/PredictiveMove/MoveableObjectType_Enum Enum"))
  (return "NewEnumerator0"))

(fn `UserConstructionScript`
  ;[1 1 1] Set the land position and dynamically spawn the mesh so it has all the materials.
  (`SceneComponent.K2_SetRelativeLocation` (`self.LandPosition`) (`self.Land Pos`) false false)
  (bind _returnvalue (`AddComponent|NODE_AddStaticMeshComponent-0`))
  (`StaticMeshComponent.SetStaticMesh` _returnvalue (`self.Static Mesh`))
  (`SceneComponent.SetRelativeScale3D` _returnvalue (`self.MeshScale`))
  (`SceneComponent.K2_SetRelativeRotation` _returnvalue (`self.MeshRotation`) false false))