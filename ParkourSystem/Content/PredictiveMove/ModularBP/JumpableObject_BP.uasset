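; JumpableObject_BP is an object in a predictive movement system that supplies the peak and landing points for the player's jump over or onto it.
; The construction script keeps the peak marker vertical-only and destroys the spline when UseSpline is off.
; Landing is the spline point closest to the player, or a fixed scene component without a spline.
; Peak XY averages the player with that spline point or the actor, using the marker's height.
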(fn `GetLandPosition`
  (returns (Location :type "Vector Structure"))
  ;[1 1 1] If using spline, get closent position to player for it. Otherwise, use the land scene component.
  (`/Engine/EditorBlueprintResources/StandardMacros.IsValid` (`self.Spline`)
    (:`Is Valid`
      (return (`SplineComponent.FindLocationClosestToWorldLocation` (`self.Spline`) (`self.K2_GetActorLocation` (`GameplayStatics.GetPlayerCharacter` 0)) "World")))
    (:`Is Not Valid`
      (return (`SceneComponent.K2_GetComponentLocation` (`self.LandPosition`))))))

(fn `GetPeakPosition`
  (returns (Location :type "Vector Structure"))
  (bind _returnvalue (`self.K2_GetActorLocation` (`GameplayStatics.GetPlayerCharacter` 0)))
  (bind (_returnvalue_x _returnvalue_y _returnvalue_z) (`KismetMathLibrary.BreakVector` (`SceneComponent.K2_GetComponentLocation` (`self.JumpPeakHeight`))))
  (bind (_returnvalue_x_2 _returnvalue_y_2) (`KismetMathLibrary.BreakVector` (`KismetMathLibrary.GetVectorArrayAverage` (`|MakeArray` (`SplineComponent.FindLocationClosestToWorldLocation` (`self.Spline`) _returnvalue "World") _returnvalue))))
  ;[1 1 1] If using spline, find average between it and the player, otherwise between this actor and the player.
  (`/Engine/EditorBlueprintResources/StandardMacros.IsValid` (`self.Spline`)
    (:`Is Valid`
      (return (`KismetMathLibrary.MakeVector` _returnvalue_x_2 _returnvalue_y_2 _returnvalue_z)))
    (:`Is Not Valid`
      (bind _returnvalue_2 (`GameplayStatics.GetActorArrayAverageLocation` (`|MakeArray` self (`GameplayStatics.GetPlayerCharacter` 0) :!type "Actor Object Reference")))
      (return (`KismetMathLibrary.MakeVector` (.x _returnvalue_2) (.y _returnvalue_2) _returnvalue_z)))))

(fn `GetSpline`
  (returns (Spline :type "SplineComponent Object Reference"))
  (return (`self.Spline`)))

(fn `GetType`
  (returns (NewParam :type "/Game/PredictiveMove/MoveableObjectType_Enum Enum"))
  (return "NewEnumerator0"))

(fn `UserConstructionScript`
  (bind (_peakheightpos_x _peakheightpos_y _peakheightpos_z) (`KismetMathLibrary.BreakVector` (`self.PeakHeightPos`)))
  ;[1 1 1] Set the peak height, and if not using spline, destroy the component.
  (`parent.UserConstructionScript`)
  (`SceneComponent.K2_SetRelativeLocation` (`self.JumpPeakHeight`) (`KismetMathLibrary.MakeVector` 0.0 0.0 _peakheightpos_z) false false)
  (set `self.PeakHeightPos` (`KismetMathLibrary.MakeVector` 0.0 0.0 _peakheightpos_z))
  (if (not (`self.UseSpline?`))
    (`ActorComponent.K2_DestroyComponent` (`self.Spline`))))